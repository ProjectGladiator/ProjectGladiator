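; BP_MyCharacter is a character Blueprint with two attacks: a missile shot and a short-range forward hit.
; Pressing R spawns a Missle actor at the Arrow1 component's transform.
; The Attack input sphere-traces ahead for pawns other than itself, with debug drawing, and passes the result to point damage without checking for a hit.
; A line-trace alternative feeding the same damage call is left disconnected.
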(event Input|ActionEvents|InputActionAttack
  (params (Key :type Key%20Structure))
  (bind _returnvalue (Transformation|GetActorLocation))
  (:Pressed
    (bind _outhit (Collision|SphereTraceForObjects _returnvalue (+ _returnvalue (* (Transformation|GetActorForwardVector) 3e+02)) 5e+01 (Utilities|Array|MakeArray "ObjectTypeQuery3") false (Utilities|Array|MakeArray self) "ForDuration" true "(R=1.000000,G=0.000000,B=0.000000,A=1.000000)" "(R=0.000000,G=1.000000,B=0.000000,A=1.000000)" 1.0))
    (Game|Damage|ApplyPointDamage (.HitActor (Collision|BreakHitResult _outhit)) 1e+01 (.ImpactPoint (Collision|BreakHitResult _outhit)) _outhit (Pawn|GetController) self)))

(event Input|KeyboardEvents|R
  (params (Key :type Key%20Structure))
  (:Pressed
    (Game|SpawnActorfromClass "/Game/Blueprints/MyCharacter/Blueprints/Missle.Missle_C" (Transformation|GetWorldTransform (Variables|Default|GetArrow1)) "AlwaysSpawn" 0 0)))

(fn ConstructionScript)